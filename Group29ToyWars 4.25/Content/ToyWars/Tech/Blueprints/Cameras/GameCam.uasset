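; Game camera actor for ToyWars that slides along the Y axis to follow the average position of spawned actors.
; Initialisation binds to the GM reference's spawn dispatcher to build a watch list, which drops actors when they are destroyed, and starts a looping timer.
; Each update averages the watched locations and plays a timeline that lerps only the camera's Y toward that average, clamped to fixed bounds.
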(event `Initialisation`
  (params (GMRef :type "/Game/ToyWars/Tech/Gamemodes/MainMenuGameModeVersion2 Object Reference"))
  ;[1 1 1] Init
  (bind _output_get (set `self.GMRef` GMRef))
  (add `/Game/ToyWars/Tech/Gamemodes/MainMenuGameModeVersion2.ActorSpawned` _output_get (`|CreateDelegate` :!event `ActorSpawned`))
  (`KismetSystemLibrary.K2_SetTimerDelegate` (`|CreateDelegate` :!event `SetCameraLocation`) 0.1 true))

(event `ActorSpawned`
  (params (ActorArray :type "Actor Object Reference"))
  ;[1 1 1] Add spawned actor to the watch list
  (`KismetArrayLibrary.Array_Add` (`self.ActorsToWatch`) ActorArray)
  (add `self.OnDestroyed` ActorArray (`|CreateDelegate` :!event `RemoveFromWatchList`)))

(event `RemoveFromWatchList` :!signature `self.OnDestroyed`
  (params (DestroyedActor :type "Actor Object Reference"))
  ;[1 1 1] Remove When destroyed
  (`KismetArrayLibrary.Array_RemoveItem` (`self.ActorsToWatch`) DestroyedActor))

(event `self.ReceiveTick`
  (params (DeltaSeconds :type "Float (single-precision)"))
  (bind (_returnvalue_x _returnvalue_y _returnvalue_z) (`KismetMathLibrary.BreakVector` (`self.K2_GetActorLocation`)))
  (bind (_returnvalue_x_2 _returnvalue_y_2 _returnvalue_z_2) (`KismetMathLibrary.BreakVector` (`self.K2_GetActorLocation`)))
  (bind (_averagevector_x _averagevector_y) (`KismetMathLibrary.BreakVector` (`self.AverageVector`)))
  (set `self.Vector` (0.0 0.0 0.0))
  (if (> (`KismetArrayLibrary.Array_Length` (`self.ActorsToWatch`)) 0)
    (for _array_element (`self.ActorsToWatch`)
      (set `self.Vector` (+ (`self.Vector`) (`self.K2_GetActorLocation` _array_element))))
    (set `self.AverageVector` (/ (`self.Vector`) (`KismetArrayLibrary.Array_Length` (`self.ActorsToWatch`))))
    (bind (_direction _speed) (`Timeline|CameraMovement`)
      (:`Update`
        (bind (_returnvalue_x_3 _returnvalue_y_3 _returnvalue_z_3) (`KismetMathLibrary.BreakVector` (`KismetMathLibrary.VLerp` (`KismetMathLibrary.MakeVector` _returnvalue_x _returnvalue_y _returnvalue_z) (`KismetMathLibrary.MakeVector` _returnvalue_x_2 _averagevector_y _returnvalue_z_2) _speed)))
        (`self.K2_SetActorLocation` (`KismetMathLibrary.MakeVector` _returnvalue_x_3 (`KismetMathLibrary.FClamp` _returnvalue_y_3 -900.0 900.0) _returnvalue_z_3))))))

(event `SetCameraLocation`)

(fn `UserConstructionScript`)