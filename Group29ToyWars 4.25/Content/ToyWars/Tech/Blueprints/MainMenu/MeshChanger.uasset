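; MeshChanger is a main-menu trigger actor that recolors the player's Body when the player overlaps its Sphere.
; The ChangeMeshToWhat enum (Boy, Girl, Cat) picks a blue, pink or green prototype material for material slot 0.
; The construction script applies the same material to the Cylinder, so the pickup previews its choice.
; Despite the name, it swaps only materials, not meshes.
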(event `self.Sphere.OnComponentBeginOverlap`
  (params (OverlappedComponent :type "PrimitiveComponent Object Reference") (OtherActor :type "Actor Object Reference") (OtherComp :type "PrimitiveComponent Object Reference") (OtherBodyIndex :type Integer) (bFromSweep :type Boolean) (SweepResult :type "HitResult Structure (by ref)"))
  (bind _asplayer (cast `/Game/Prototype/Blueprints/Tom/Player/BP_Player/Blueprints/Player` OtherActor))
  (switch `/Game/ToyWars/Tech/Blueprints/Enums/BoyGirl` (`self.ChangeMeshToWhat`)
    (:`NewEnumerator0`
      (bind _body (`/Game/Prototype/Blueprints/Tom/Player/BP_Player/Blueprints/Player.Body` _asplayer))
      (`PrimitiveComponent.SetMaterial` _body 0 "/Game/ToyWars/Art/_Placeholder_/Materials/Prototype/Proto_Blue.Proto_Blue"))
    (:`NewEnumerator1`
      (`PrimitiveComponent.SetMaterial` _body 0 "/Game/ToyWars/Art/_Placeholder_/Materials/Prototype/Proto_Pink.Proto_Pink"))
    (:`NewEnumerator2`
      (`PrimitiveComponent.SetMaterial` _body 0 "/Game/ToyWars/Art/_Placeholder_/Materials/Prototype/Proto_Green.Proto_Green"))))

(fn `UserConstructionScript`
  (bind _cylinder (`self.Cylinder`))
  (switch `/Game/ToyWars/Tech/Blueprints/Enums/BoyGirl` (`self.ChangeMeshToWhat`)
    (:`NewEnumerator0`
      (`PrimitiveComponent.SetMaterial` _cylinder 0 "/Game/ToyWars/Art/_Placeholder_/Materials/Prototype/Proto_Blue.Proto_Blue"))
    (:`NewEnumerator1`
      (`PrimitiveComponent.SetMaterial` _cylinder 0 "/Game/ToyWars/Art/_Placeholder_/Materials/Prototype/Proto_Pink.Proto_Pink"))
    (:`NewEnumerator2`
      (`PrimitiveComponent.SetMaterial` _cylinder 0 "/Game/ToyWars/Art/_Placeholder_/Materials/Prototype/Proto_Green.Proto_Green"))))