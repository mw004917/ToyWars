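; BaseBear is an AI-controlled team unit that attacks enemies, takes damage and carries a target base to attack.
; On possession it creates a BearHealthBar widget bound to itself.
; Attack applies damage to actors overlapping its sphere whose team differs from its own.
; Damage briefly flashes the mesh red, and at zero health it stops AI logic, fires a destroyed call and destroys itself after a delay.
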(event `self.ReceivePossessed`
  (params (NewController :type "Controller Object Reference"))
  (bind _returnvalue (`|CreateWidget` "/Game/ToyWars/Tech/UI/Bear/BearHealthBar.BearHealthBar_C"))
  (`/Game/ToyWars/Tech/UI/Bear/BearHealthBar.InitialisationW` _returnvalue self)
  (`WidgetComponent.SetWidget` (`self.Widget`) _returnvalue))

(event `/Game/ToyWars/Tech/Blueprints/Interfaces/GetPerceptionComponent.Attack`
  (for _array_element (`PrimitiveComponent.GetOverlappingActors` (`self.Sphere`) null)
    (bind _output_get (set `self.ActorInDamageRadius` _array_element))
    (bind _team (message `/Game/ToyWars/Tech/Blueprints/Interfaces/GetTeam.GetTeam` _output_get))
    (if (!= _team (`self.Team`))
      (`GameplayStatics.ApplyDamage` (`self.ActorInDamageRadius`) (`self.BearDamage`)))))

(event `/Game/ToyWars/Tech/Blueprints/Interfaces/GetTeam.SetBaseToAttack`
  (params (BaseToAttack :type "/Game/ToyWars/Tech/Blueprints/TeamBase/TeamBase_BP Object Reference"))
  (set `self.BaseTarget` BaseToAttack))

(event `/Game/ToyWars/Tech/Blueprints/Interfaces/GetTeam.SetTeam`
  (params (TeamToBe :type "/Game/ToyWars/Tech/Blueprints/Enums/Team Enum" :default "NewEnumerator0"))
  (set `self.Team` TeamToBe))

(event `self.ReceiveAnyDamage`
  (params (Damage :type "Float (single-precision)") (DamageType :type "DamageType Object Reference") (InstigatedBy :type "Controller Object Reference") (DamageCauser :type "Actor Object Reference"))
  (bind _output_get (set `self.Health` (- (`self.Health`) Damage)))
  (if (<= _output_get 0.0)
    (set `self.Health` 0.0)
    (`/Engine/EditorBlueprintResources/StandardMacros.DoOnce` false
      (:`Completed`
        (`BrainComponent.StopLogic` (`AIController.BrainComponent` (`AIBlueprintHelperLibrary.GetAIController` self)) "")
        (`self.DestroyedCall`)
        (`KismetSystemLibrary.Delay` 1.0)
        (`self.K2_DestroyActor`)))
    (else
      (`self.HealthUpdatedCall`)
      (`PrimitiveComponent.SetMaterial` (`self.Mesh`) 1 "/Game/ToyWars/Art/_Placeholder_/Materials/Prototype/Proto_Red.Proto_Red")
      (`PrimitiveComponent.SetMaterial` (`self.Mesh`) 0 "/Game/ToyWars/Art/_Placeholder_/Materials/Prototype/Proto_Red.Proto_Red")
      (`KismetSystemLibrary.Delay` 1.0)
      (`PrimitiveComponent.SetMaterial` (`self.Mesh`) 1 "/Game/ToyWars/Tech/_Placeholder_/Mannequin/Character/Materials/M_UE4Man_ChestLogo.M_UE4Man_ChestLogo")
      (`PrimitiveComponent.SetMaterial` (`self.Mesh`) 0 "/Game/ToyWars/Tech/_Placeholder_/Mannequin/Character/Materials/M_UE4Man_Body.M_UE4Man_Body"))))

(fn `GetBaseToAttack`
  (returns (BaseToAttack :type "/Game/ToyWars/Tech/Blueprints/TeamBase/TeamBase_BP Object Reference"))
  (return (`self.BaseTarget`)))

(fn `GetHealth`
  (returns (HealthInHere :type "Float (double-precision)"))
  (return (`self.Health`)))

(fn `GetPerceptionComponent`
  (returns (ComponentInHere :type "AIPerceptionComponent Object Reference"))
  (return (`self.AIPerception`)))

(fn `GetTeam`
  (returns (Team :type "/Game/ToyWars/Tech/Blueprints/Enums/Team Enum"))
  (return (`self.Team`)))

(fn `UserConstructionScript`)