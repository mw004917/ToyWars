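; Team base actor for Toy Wars: a destructible base that spawns AI bears to attack the enemy base.
; Damage lowers its health and fires health-changed or one-time destroyed dispatchers, with a particle burst on destruction; a widget health bar receives a base reference.
; Spawn creates behavior-tree bears at random points within SpawnBox, passing each its team and enemy base.
; The construction script colors the mesh by team.
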(event `self.ReceiveBeginPlay`
  ;[1 1 1] Init
  (`self.Initalisation`))

(event `Initalisation`
  ;[1 1 1] Init
  (bind _returnvalue (`|CreateWidget` "/Game/ToyWars/Tech/UI/BaseHealthBar.BaseHealthBar_C"))
  (`WidgetComponent.SetWidget` (`self.Widget`) _returnvalue)
  (`/Game/ToyWars/Tech/UI/BaseHealthBar.Initialisation` _returnvalue self))

(event `self.ReceiveAnyDamage`
  (params (Damage :type "Float (single-precision)") (DamageType :type "DamageType Object Reference") (InstigatedBy :type "Controller Object Reference") (DamageCauser :type "Actor Object Reference"))
  ;[1 1 1] Damage and Death
  (bind _output_get (set `self.TeamBaseHealth` (- (`self.TeamBaseHealth`) Damage)))
  (if (<= _output_get 0.0)
    (set `self.TeamBaseHealth` 0.0)
    (`/Engine/EditorBlueprintResources/StandardMacros.DoOnce` false
      (:`Completed`
        (`self.BaseDestroyed`)
        (`GameplayStatics.SpawnEmitterAtLocation` "/Engine/Tutorial/SubEditors/TutorialAssets/TutorialParticleSystem.TutorialParticleSystem" (`self.K2_GetActorLocation`))))
    (else
      (`self.HealthChanged`))))

(event `/Game/ToyWars/Tech/Blueprints/Interfaces/GetTeam.SetTeam`
  (params (TeamToBe :type "/Game/ToyWars/Tech/Blueprints/Enums/Team Enum" :default "NewEnumerator0"))
  ;[1 1 1] Set Team Functionality
  (set `self.Team` TeamToBe))

(event `/Game/Prototype/Blueprints/Tom/BearConstructionStation/Spawn.Spawn`
  (bind _spawnbox (`self.SpawnBox`))
  (bind (_returnvalue_x _returnvalue_y) (`KismetMathLibrary.BreakVector` (`KismetMathLibrary.RandomPointInBoundingBox` (`SceneComponent.K2_GetComponentLocation` _spawnbox) (`BoxComponent.BoxExtent` _spawnbox))))
  ;[1 1 1] Interface Maybe ?
  ;[1 1 1] Spawn a Bear
  (for _ (range (+ (`self.SpawnThisNoOfBears`) 1))
    (bind _returnvalue (`AIBlueprintHelperLibrary.SpawnAIFromClass` "/Game/ToyWars/Tech/Blueprints/Character/BaseBear.BaseBear_C" "/Game/ToyWars/Tech/AI/BT_BaseBear.BT_BaseBear" (`KismetMathLibrary.MakeVector` _returnvalue_x _returnvalue_y -300.0) (`SceneComponent.K2_GetComponentRotation` (`self.Arrow`)) true null))
    (message `/Game/ToyWars/Tech/Blueprints/Interfaces/GetTeam.SetTeam` _returnvalue (`self.Team`))
    (message `/Game/ToyWars/Tech/Blueprints/Interfaces/GetTeam.SetBaseToAttack` _returnvalue (`self.EnemyBaseRef`))
    (`Controller.Possess` (`AIBlueprintHelperLibrary.GetAIController` _returnvalue) _returnvalue)))

(fn `GetBaseToAttack`
  (returns (BaseToAttack :type "/Game/ToyWars/Tech/Blueprints/TeamBase/TeamBase_BP Object Reference"))
  (return null))

(fn `GetTeam`
  (returns (Team :type "/Game/ToyWars/Tech/Blueprints/Enums/Team Enum"))
  (return (`self.Team`)))

(fn `UserConstructionScript`
  (switch `/Game/ToyWars/Tech/Blueprints/Enums/Team` (`self.Team`)
    (:`NewEnumerator0`
      (set `self.BaseMaterial` "/Game/ToyWars/Tech/Materials/Prototype/Proto_Yellow.Proto_Yellow"))
    (:`NewEnumerator1`
      (set `self.BaseMaterial` "/Game/ToyWars/Tech/Materials/Prototype/Proto_Red.Proto_Red")))
  (`PrimitiveComponent.SetMaterial` (`self.StaticMesh`) 0 (`self.BaseMaterial`)))