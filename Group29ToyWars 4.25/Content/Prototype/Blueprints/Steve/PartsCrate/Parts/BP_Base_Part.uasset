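; Base Blueprint for a part that can be thrown, picked up by an activator or delivered to a receiver.
; Throw turns on mesh physics and applies an impulse, while a delayed toggle controls trigger overlaps, with only the player trigger switched off on disable.
; The player trigger offers activation via I_Activator, handing over PartType on pickup.
; The world trigger passes PartType to I_RecievePart actors, and the part destroys itself once taken or accepted.
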(event `self.ReceiveBeginPlay`
  (`self.DisableTrigger`))

(event `/Game/Prototype/Blueprints/Steve/PartsCrate/Parts/I_Part.TogglePlayerTrigger`
  (params (Toggle :type Boolean) (Delay :type "Float (single-precision)"))
  (`KismetSystemLibrary.Delay` Delay)
  (if Toggle
    (`self.EnableTrigger`)
    (else
      (`self.DisableTrigger`))))

(event `EnableTrigger`
  (set `PrimitiveComponent.bGenerateOverlapEvents` true (`self.Tigger_Player`))
  (set `PrimitiveComponent.bGenerateOverlapEvents` true (`self.Tigger_WorldDynamic`)))

(event `DisableTrigger`
  (set `PrimitiveComponent.bGenerateOverlapEvents` false (`self.Tigger_Player`)))

(event `/Game/Prototype/Blueprints/Steve/PartsCrate/Parts/I_Throwable.Throw`
  (params (ThrowDir :type "Vector Structure") (ThrowPower :type "Float (single-precision)"))
  (`PrimitiveComponent.SetSimulatePhysics` (`self.Part_Mesh`) true)
  (`PrimitiveComponent.SetCollisionProfileName` (`self.Part_Mesh`) "BlockAll" true)
  (`PrimitiveComponent.AddImpulse` (`self.Part_Mesh`) (* ThrowDir (* 100 ThrowPower)) "None" true))

(event `self.Tigger_Player.OnComponentBeginOverlap`
  (params (OverlappedComponent :type "PrimitiveComponent Object Reference") (OtherActor :type "Actor Object Reference") (OtherComp :type "PrimitiveComponent Object Reference") (OtherBodyIndex :type Integer) (bFromSweep :type Boolean) (SweepResult :type "HitResult Structure (by ref)"))
  (if (`KismetSystemLibrary.DoesImplementInterface` OtherActor "/Game/Prototype/Blueprints/Steve/PartsCrate/I_Activator.I_Activator_C")
    (message `/Game/Prototype/Blueprints/Steve/PartsCrate/I_Activator.SetActivatable` OtherActor self)))

(event `self.Tigger_Player.OnComponentEndOverlap`
  (params (OverlappedComponent :type "PrimitiveComponent Object Reference") (OtherActor :type "Actor Object Reference") (OtherComp :type "PrimitiveComponent Object Reference") (OtherBodyIndex :type Integer))
  (if (`KismetSystemLibrary.DoesImplementInterface` OtherActor "/Game/Prototype/Blueprints/Steve/PartsCrate/I_Activator.I_Activator_C")
    (message `/Game/Prototype/Blueprints/Steve/PartsCrate/I_Activator.ClearActivatable` OtherActor)))

(event `/Game/Prototype/Blueprints/Steve/PartsCrate/I_Activatable.Activate`
  (params (Activator :type "/Game/Prototype/Blueprints/Tom/Player/BP_Player/Blueprints/Player Object Reference"))
  (`/Game/Prototype/Blueprints/Tom/Player/BP_Player/Blueprints/Player.Part_Pickup` Activator (`self.PartType`))
  (message `/Game/Prototype/Blueprints/Steve/PartsCrate/I_Activator.ClearActivatable` Activator)
  (`self.K2_DestroyActor`))

(event `self.Tigger_WorldDynamic.OnComponentBeginOverlap`
  (params (OverlappedComponent :type "PrimitiveComponent Object Reference") (OtherActor :type "Actor Object Reference") (OtherComp :type "PrimitiveComponent Object Reference") (OtherBodyIndex :type Integer) (bFromSweep :type Boolean) (SweepResult :type "HitResult Structure (by ref)"))
  (if (`KismetSystemLibrary.DoesImplementInterface` OtherActor "/Game/Prototype/Blueprints/Steve/PartsCrate/Parts/I_RecievePart.I_RecievePart_C")
    (bind _success (message `/Game/Prototype/Blueprints/Steve/PartsCrate/Parts/I_RecievePart.RecievePart` OtherActor (`self.PartType`)))
    (if _success
      (`self.OnRecieved`)
      (`self.K2_DestroyActor`))))

(fn `UserConstructionScript`)