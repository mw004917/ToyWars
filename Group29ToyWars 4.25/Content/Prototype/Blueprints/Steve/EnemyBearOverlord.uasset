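; EnemyBearOverlord is a prototype spawner that sends enemy bears down two lanes.
; Five seconds after BeginPlay it spawns the first bear, then a looping timer calls SpawnBear at a fixed interval.
; Each spawn randomly picks one of two spawn points, faces the bear along its forward vector and passes the matching lane target, enemy team ID and a preset body-part loadout with a sword.
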(event `self.ReceiveBeginPlay`
  (`KismetSystemLibrary.Delay` 5.0)
  (`self.SpawnBear`)
  (`KismetSystemLibrary.K2_SetTimer` null "SpawnBear" 20.0 true))

(fn `SpawnBear`
  (locals (LaneID :type Integer :default 0) (SpawnLocation :type "Vector Structure") (SpawnRotation :type "Rotator Structure") (LaneTarget :type "/Game/Prototype/Blueprints/Tom/Bear/LaneTargetPoint Object Reference"))
  (bind _output_get (set `local.LaneID` (`KismetMathLibrary.RandomIntegerInRange` 0 1)))
  (switch `int` _output_get
    (:`0`
      (set `local.SpawnLocation` (`SceneComponent.K2_GetComponentLocation` (`self.SpawnPoint_1`)))
      (set `local.SpawnRotation` (`KismetMathLibrary.MakeRotFromX` (`SceneComponent.GetForwardVector` (`self.SpawnPoint_1`))))
      (set `local.LaneTarget` (`self.Lane1_Target`)))
    (:`1`
      (set `local.SpawnRotation` (`KismetMathLibrary.MakeRotFromX` (`SceneComponent.GetForwardVector` (`self.SpawnPoint_2`))))
      (set `local.SpawnLocation` (`SceneComponent.K2_GetComponentLocation` (`self.SpawnPoint_2`)))
      (set `local.LaneTarget` (`self.Lane2_Target`))))
  (`|SpawnActorFromClass` "/Game/Prototype/Blueprints/Tom/Bear/Bear.Bear_C" (`KismetMathLibrary.MakeTransform` (`local.SpawnLocation`) (`local.SpawnRotation`)) "AlwaysSpawn" "OverrideRootScale" null 1 (`local.LaneTarget`) (`|MakeMap` "NewEnumerator5" null "NewEnumerator4" null "NewEnumerator3" "/Game/Prototype/Blueprints/Steve/PartsCrate/Parts/BP_Part_Sword.BP_Part_Sword_C" "NewEnumerator2" "/Game/Prototype/Blueprints/Steve/PartsCrate/Parts/BP_Part_Legs.BP_Part_Legs_C" "NewEnumerator1" "/Game/Prototype/Blueprints/Steve/PartsCrate/Parts/BP_Part_Torso.BP_Part_Torso_C" "NewEnumerator0" "/Game/Prototype/Blueprints/Steve/PartsCrate/Parts/BP_Part_Head.BP_Part_Head_C" :!type "/Game/Prototype/Blueprints/Steve/PartsCrate/PartTypes Enum" :!valuetype "Actor Class Reference") null))

(fn `UserConstructionScript`)