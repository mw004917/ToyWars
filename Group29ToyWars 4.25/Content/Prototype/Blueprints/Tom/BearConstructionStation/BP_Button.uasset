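; BP_Button is a prototype button for the bear construction station that tells a referenced spawner to spawn when triggered.
; An overlap on its box by an actor implementing the PickUp interface passes a DoOnce gate and calls SpawnMessage, then re-arms after a short delay.
; A dynamic material created on BeginPlay lets Toggle_ButtonFlash switch the cube's flashing on or off through a FlashRate parameter.
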(event `Toggle_ButtonFlash`
  (params (Toggle :type Boolean))
  (if Toggle
    (`MaterialInstanceDynamic.SetScalarParameterValue` (`self.mat_button`) "FlashRate" 1.0)
    (else
      (`MaterialInstanceDynamic.SetScalarParameterValue` (`self.mat_button`) "FlashRate" 0.0))))

(event `self.ReceiveBeginPlay`
  (bind _returnvalue (`KismetMaterialLibrary.CreateDynamicMaterialInstance` "/Game/Prototype/Blueprints/Tom/BearConstructionStation/Mat_Button.Mat_Button"))
  (bind _output_get (set `self.mat_button` _returnvalue))
  (`PrimitiveComponent.SetMaterial` (`self.Cube`) 0 _output_get))

(event `Reset`
  (goto _label :!via `Reset`))

(event `self.Box.OnComponentBeginOverlap`
  (params (OverlappedComponent :type "PrimitiveComponent Object Reference") (OtherActor :type "Actor Object Reference") (OtherComp :type "PrimitiveComponent Object Reference") (OtherBodyIndex :type Integer) (bFromSweep :type Boolean) (SweepResult :type "HitResult Structure (by ref)"))
  (if (`KismetSystemLibrary.DoesImplementInterface` OtherActor "/Game/Prototype/Blueprints/Tom/Player/PickUp.PickUp_C")
    (`/Engine/EditorBlueprintResources/StandardMacros.DoOnce` false :!label _label
      (:`Completed`
        (message `/Game/Prototype/Blueprints/Tom/BearConstructionStation/Spawn.Spawn` (`self.SpawnerRef`))
        (`KismetSystemLibrary.Delay` 2.0)
        (`self.Reset`)))))

(fn `UserConstructionScript`)