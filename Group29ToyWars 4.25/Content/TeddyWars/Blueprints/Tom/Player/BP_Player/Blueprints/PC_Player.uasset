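; Player controller for TeddyWars that manages the tutorial, main UI, respawning and game-over flow.
; On BeginPlay it caches the first PlayerSpawnPoint and, for controller ID 0, shows the tutorial with the game paused.
; Go unpauses and adds the master UI, Respawn teleports the pawn to that spawn, and Gameover forwards the result to the UI.
; Reset opens FinnDeliverableMap when the GameMode's game-over message flag is set.
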(event `self.ReceiveBeginPlay`
  (bind _outactors (`GameplayStatics.GetAllActorsOfClass` "/Game/TeddyWars/Blueprints/Tom/Player/BP_Player/Blueprints/PlayerSpawnPoint.PlayerSpawnPoint_C"))
  (set `self.SpawnPoint` (`|GetArrayItem` _outactors))
  (if (== (`GameplayStatics.GetPlayerControllerID` self) 0)
    (`GameplayStatics.SetGamePaused` false)
    (set `self.bShowMouseCursor` true)
    (bind _returnvalue (`|CreateWidget` "/Game/TeddyWars/Blueprints/Tom/UI/Tutorial/TutorialWidget.TutorialWidget_C" null self))
    (`UserWidget.AddToViewport` _returnvalue 0)
    (`GameplayStatics.SetGamePaused` true)))

(event `Go`
  (`GameplayStatics.SetGamePaused` false)
  (bind _returnvalue (`|CreateWidget` "/Game/TeddyWars/Blueprints/Steve/UI/MasterUI.MasterUI_C" self))
  (bind _output_get (set `self.UI` _returnvalue))
  (`UserWidget.AddToViewport` _output_get 0))

(event `/Game/TeddyWars/Blueprints/Tom/Player/BP_Player/Blueprints/I_PCP.Respawn`
  (`self.K2_SetActorLocation` (`self.K2_GetPawn`) (`self.K2_GetActorLocation` (`self.SpawnPoint`)) false false))

(event `/Game/TeddyWars/Blueprints/Tom/Player/BP_Player/Blueprints/I_PCP.Gameover`
  (params (HasWon :type Boolean))
  (`/Game/TeddyWars/Blueprints/Steve/UI/MasterUI.GameOver` (`self.UI`) HasWon))

(event `InputAction|Reset` :paused true
  (params (Key :type "Key Structure"))
  (:`Pressed`
    (bind _isgameover (message `/Game/TeddyWars/Blueprints/Steve/Gamemode/I_GMTeddy.GetIsGameOver` (`GameplayStatics.GetGameMode`)))
    (if _isgameover
      (`GameplayStatics.OpenLevel` "FinnDeliverableMap"))))

(fn `UserConstructionScript`)