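; BP_Train is a train that runs along a referenced track spline and knocks players out of its way.
; A slowed timeline maps 0-1 progress to spline distance, setting location and rotation each update.
; A FlipFlop on completion first reports arrival to the parent manager, waits, then reverses, and next time has the manager replace the train.
; Mesh hit or overlap launches the Player with a fixed velocity.
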(event `self.ReceiveBeginPlay`
  (`self.AllAboard`))

(event `AllAboard`
  (bind _parentmanager (`self.ParentManager`))
  (bind _spline (`/Game/TeddyWars/Blueprints/Tom/Train/TrainTracks.Spline` (`self.TrackRef`)))
  (set `self.NewPlayRate` (/ 1.0 15.0))
  (`TimelineComponent.SetPlayRate` (`self.Timeline_0`) (`self.NewPlayRate`))
  (bind (_direction _newtrack_0) (`Timeline|Timeline_0` :!label _label)
    (:`Update`
      (bind _returnvalue (* _newtrack_0 (`SplineComponent.GetSplineLength` _spline)))
      (`self.K2_SetActorLocation` (`SplineComponent.GetLocationAtDistanceAlongSpline` _spline _returnvalue "World"))
      (`self.K2_SetActorRotation` (`SplineComponent.GetRotationAtDistanceAlongSpline` (`/Game/TeddyWars/Blueprints/Tom/Train/TrainTracks.Spline` (`self.TrackRef`)) _returnvalue "World")))
    (:`Finished`
      (`/Engine/EditorBlueprintResources/StandardMacros.FlipFlop`
        (:`A`
          (`/Game/TeddyWars/Blueprints/Tom/Train/TrainManager.Arrived` _parentmanager)
          (`KismetSystemLibrary.Delay` 10.0)
          (`/Game/TeddyWars/Blueprints/Tom/Train/TrainManager.Reverse` _parentmanager)
          (goto _label :!via `Reverse`))
        (:`B`
          (`/Game/TeddyWars/Blueprints/Tom/Train/TrainManager.DeleteTrain And spawn another` _parentmanager))))))

(event `self.StaticMesh.OnComponentHit`
  (params (HitComponent :type "PrimitiveComponent Object Reference") (OtherActor :type "Actor Object Reference") (OtherComp :type "PrimitiveComponent Object Reference") (NormalImpulse :type "Vector Structure") (Hit :type "HitResult Structure (by ref)"))
  (bind _asplayer (cast `/Game/TeddyWars/Blueprints/Tom/Player/BP_Player/Blueprints/Player` (stale `self.StaticMesh.OnComponentBeginOverlap` OtherActor) :!label _label_2))
  (`Character.LaunchCharacter` _asplayer (250.0 250.0 125.0) true true))

(event `self.StaticMesh.OnComponentBeginOverlap`
  (params (OverlappedComponent :type "PrimitiveComponent Object Reference") (OtherActor :type "Actor Object Reference") (OtherComp :type "PrimitiveComponent Object Reference") (OtherBodyIndex :type Integer) (bFromSweep :type Boolean) (SweepResult :type "HitResult Structure (by ref)"))
  (goto _label_2))

(fn `UserConstructionScript`)