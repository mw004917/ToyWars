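; Bear construction station where delivered parts are assembled into a bear for a team.
; RecievePart accepts head, torso, legs and only one of sword, armor or bow, displaying each through a Child Actor Component and recording it in CurParts.
; A complete set sets BearReady and flashes the button.
; Spawn calls SpawnBear on the team base without passing parts, fires OnSpawn and resets the station; the direct SpawnActor path is disconnected.
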(event `self.ReceiveBeginPlay`
  ;[1 1 1] Init
  (set `self.PartCACs` (`|MakeArray` (`self.CA_Head`) (`self.CA_Torso`) (`self.CA_Leg`) (`self.CA_Sword`) (`self.CA_Armor`) (`self.CA_Bow`))))

(event `/Game/TeddyWars/Blueprints/Tom/BearConstructionStation/Spawn.Spawn`
  ;[1 1 1] Bear Spawning Logic
  (`/Game/TECH/BLUEPRINTS/TeamBase/TeamBase_BP.SpawnBear` (`self.TeamBaseToSpawnAt`))
  (set `self.BearReady?` false)
  (`self.OnSpawn`)
  (set `self.CurParts` (`|MakeMap` "NewEnumerator5" null "NewEnumerator4" null "NewEnumerator3" null "NewEnumerator2" null "NewEnumerator1" null "NewEnumerator0" :!type "/Game/TeddyWars/Blueprints/Steve/PartsCrate/PartTypes Enum" :!valuetype "Actor Class Reference"))
  (`/Game/TeddyWars/Blueprints/Tom/BearConstructionStation/BP_Button.Toggle_ButtonFlash` (`self.Button`) false)
  (for _array_element (`self.PartCACs`)
    (`ChildActorComponent.SetChildActorClass` _array_element null)))

(fn `CheckBearReady`
  (if (and (and (`KismetSystemLibrary.IsValidClass` (`BlueprintMapLibrary.Map_Find` (`self.CurParts`) "NewEnumerator0")) (`KismetSystemLibrary.IsValidClass` (`BlueprintMapLibrary.Map_Find` (`self.CurParts`) "NewEnumerator1")) (`KismetSystemLibrary.IsValidClass` (`BlueprintMapLibrary.Map_Find` (`self.CurParts`) "NewEnumerator2"))) (or (`KismetSystemLibrary.IsValidClass` (`BlueprintMapLibrary.Map_Find` (`self.CurParts`) "NewEnumerator3")) (`KismetSystemLibrary.IsValidClass` (`BlueprintMapLibrary.Map_Find` (`self.CurParts`) "NewEnumerator4")) (`KismetSystemLibrary.IsValidClass` (`BlueprintMapLibrary.Map_Find` (`self.CurParts`) "NewEnumerator5"))))
    ;[1 1 1] Set Different class mesh here before spawn
    (set `self.BearReady?` true)
    (`/Game/TeddyWars/Blueprints/Tom/BearConstructionStation/BP_Button.Toggle_ButtonFlash` (`self.Button`) true)))

(fn `RecievePart`
  (params (PartType :type "/Game/TeddyWars/Blueprints/Steve/PartsCrate/PartTypes Enum" :default "NewEnumerator0"))
  (returns (Success :type Boolean))
  (locals (IPartType :type "/Game/TeddyWars/Blueprints/Steve/PartsCrate/PartTypes Enum" :default "NewEnumerator0"))
  (bind _output (`|GetArrayItem` (`|MakeArray` "/Game/TeddyWars/Blueprints/Steve/PartsCrate/Parts/BP_Part_Head.BP_Part_Head_C" "/Game/TeddyWars/Blueprints/Steve/PartsCrate/Parts/BP_Part_Torso.BP_Part_Torso_C" "/Game/TeddyWars/Blueprints/Steve/PartsCrate/Parts/BP_Part_Legs.BP_Part_Legs_C" "/Game/TeddyWars/Blueprints/Steve/PartsCrate/Parts/BP_Part_Sword.BP_Part_Sword_C" "/Game/TeddyWars/Blueprints/Steve/PartsCrate/Parts/BP_Part_Armor.BP_Part_Armor_C" "/Game/TeddyWars/Blueprints/Steve/PartsCrate/Parts/BP_Part_Bow.BP_Part_Bow_C" :!type "Actor Class Reference") (`KismetMathLibrary.Conv_ByteToInt` (`local.IPartType`))))
  (bind _output_get (set `local.IPartType` PartType))
  (`self.CanRecievePart` _output_get
    (:`True`
      (`ChildActorComponent.SetChildActorClass` (`|GetArrayItem` (`self.PartCACs`) (`KismetMathLibrary.Conv_ByteToInt` (`local.IPartType`))) _output)
      (`BlueprintMapLibrary.Map_Add` (`self.CurParts`) (`local.IPartType`) _output)
      (`self.CheckBearReady`)
      (return true))
    (:`False`
      (return false))))

(fn `UserConstructionScript`)