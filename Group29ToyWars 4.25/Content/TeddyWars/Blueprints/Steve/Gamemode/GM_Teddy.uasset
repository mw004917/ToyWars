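; GM_Teddy is the Teddy Wars game mode that decides when a match is won or lost by tracking destroyed bases.
; On BeginPlay it binds to the death event on every Base's Health and creates an additional local player.
; Deaths are counted per TeamID; when either team loses two bases, it shows a win or loss message through the first player controller, pauses and flags game over.
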(event `self.ReceiveBeginPlay`
  (bind _outactors (`GameplayStatics.GetAllActorsOfClass` "/Game/TeddyWars/Blueprints/Steve/Base/Base.Base_C"))
  (for _array_element _outactors
    (add `/Game/TeddyWars/Blueprints/Hamish/Character/Health.DeathEvent` (`/Game/TeddyWars/Blueprints/Steve/Base/Base.Health` _array_element) (`|CreateDelegate` :!event `GM_Teddy_AutoGenFunc`)))
  (`GameplayStatics.CreatePlayer` -1))

(fn `GetIsGameOver`
  (returns (IsGameOver :type Boolean))
  (return (`self.IsGameOver`)))

(fn `GM_Teddy_AutoGenFunc`
  (params (Actor :type "Actor Object Reference"))
  (bind _asbase (cast `/Game/TeddyWars/Blueprints/Steve/Base/Base` Actor))
  (switch `int` (`/Game/TeddyWars/Blueprints/Steve/Base/Base.TeamID` _asbase)
    (:`0`
      (`/Engine/EditorBlueprintResources/StandardMacros.IncrementInt` (`self.NumPlayerBasesDead`)
        (:`  `
          (if (== (`self.NumPlayerBasesDead`) 2)
            (message `/Game/TeddyWars/Blueprints/Tom/Player/BP_Player/Blueprints/I_PCP.Gameover` (`GameplayStatics.GetPlayerController` 0) false)
            (`GameplayStatics.SetGamePaused` true :!label _label)
            (set `self.IsGameOver` true)))))
    (:`1`
      (`/Engine/EditorBlueprintResources/StandardMacros.IncrementInt` (`self.NumEnemyBasesDead`)
        (:`  `
          (if (== (`self.NumEnemyBasesDead`) 2)
            (message `/Game/TeddyWars/Blueprints/Tom/Player/BP_Player/Blueprints/I_PCP.Gameover` (`GameplayStatics.GetPlayerController` 0) true)
            (goto _label)))))))

(fn `UserConstructionScript`)