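; BP_PartsCrate is a pickup station that displays a part (head, torso, legs, sword, armor or bow) and offers that part type to players.
; Construction picks the child actor class from PartType; at play start its trigger is disabled and an optional timer spins it.
; An overlapping I_Activator registers the crate as activatable and enlarges the part until it leaves.
; Activate sends the PartType back to the activator as a pickup message.
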(event `self.ReceiveBeginPlay`
  ;[1 1 1] Init
  (`self.SetupSpin`)
  (bind _asbp_base_part (cast `/Game/TeddyWars/Blueprints/Steve/PartsCrate/Parts/BP_Base_Part` (`ChildActorComponent.ChildActor` (`self.ChildActor`))))
  (`/Game/TeddyWars/Blueprints/Steve/PartsCrate/Parts/BP_Base_Part.DisableTrigger` _asbp_base_part))

(event `self.Trigger_Player.OnComponentBeginOverlap`
  (params (OverlappedComponent :type "PrimitiveComponent Object Reference") (OtherActor :type "Actor Object Reference") (OtherComp :type "PrimitiveComponent Object Reference") (OtherBodyIndex :type Integer) (bFromSweep :type Boolean) (SweepResult :type "HitResult Structure (by ref)"))
  ;[1 1 1] Activating Logic
  (if (`KismetSystemLibrary.DoesImplementInterface` OtherActor "/Game/TeddyWars/Blueprints/Steve/PartsCrate/I_Activator.I_Activator_C")
    (if (not (`self.IsInUse`))
      (message `/Game/TeddyWars/Blueprints/Steve/PartsCrate/I_Activator.SetActivatable` OtherActor self)
      (`self.Toggle_InUse` true))))

(event `self.Trigger_Player.OnComponentEndOverlap`
  (params (OverlappedComponent :type "PrimitiveComponent Object Reference") (OtherActor :type "Actor Object Reference") (OtherComp :type "PrimitiveComponent Object Reference") (OtherBodyIndex :type Integer))
  ;[1 1 1] Activating Logic
  (if (`KismetSystemLibrary.DoesImplementInterface` OtherActor "/Game/TeddyWars/Blueprints/Steve/PartsCrate/I_Activator.I_Activator_C")
    (message `/Game/TeddyWars/Blueprints/Steve/PartsCrate/I_Activator.ClearActivatable` OtherActor)
    (if (`self.IsInUse`)
      (`self.Toggle_InUse` false))))

(event `/Game/TeddyWars/Blueprints/Steve/PartsCrate/I_Activatable.Activate`
  (params (Activator :type "/Game/TeddyWars/Blueprints/Tom/Player/BP_Player/Blueprints/Player Object Reference"))
  ;[1 1 1] Activating Logic
  (message `/Game/TeddyWars/Blueprints/Tom/Player/PickUp.Part_Pickup` Activator (`self.PartType`)))

(fn `SetupSpin`
  (if (`self.SpinObject`)
    (`KismetSystemLibrary.K2_SetTimer` null "Spin" 0.05 true)))

(fn `Spin`
  (`SceneComponent.K2_AddRelativeRotation` (`self.ChildActor`) (`KismetMathLibrary.MakeRotator` 0.0 0.0 (`self.SpinRate`)) false false))

(fn `Toggle_InUse`
  (params (InUse :type Boolean))
  (bind _output_get (set `self.IsInUse` InUse))
  (if _output_get
    (`SceneComponent.SetRelativeScale3D` (`self.ChildActor`) (2.0 2.0 2.0))
    (else
      (`SceneComponent.SetRelativeScale3D` (`self.ChildActor`) (1.0 1.0 1.0))
      (switch `/Game/TeddyWars/Blueprints/Steve/PartsCrate/PartTypes` (`self.PartType`)
        (:`NewEnumerator0`
          (`SceneComponent.SetRelativeScale3D` (`self.ChildActor`) (0.8 0.8 0.8)))))))

(fn `UserConstructionScript`
  (`ChildActorComponent.SetChildActorClass` (`self.ChildActor`) (`|GetArrayItem` (`|MakeArray` "/Game/TeddyWars/Blueprints/Steve/PartsCrate/Parts/BP_Part_Head.BP_Part_Head_C" "/Game/TeddyWars/Blueprints/Steve/PartsCrate/Parts/BP_Part_Torso.BP_Part_Torso_C" "/Game/TeddyWars/Blueprints/Steve/PartsCrate/Parts/BP_Part_Legs.BP_Part_Legs_C" "/Game/TeddyWars/Blueprints/Steve/PartsCrate/Parts/BP_Part_Sword.BP_Part_Sword_C" "/Game/TeddyWars/Blueprints/Steve/PartsCrate/Parts/BP_Part_Armor.BP_Part_Armor_C" "/Game/TeddyWars/Blueprints/Steve/PartsCrate/Parts/BP_Part_Bow.BP_Part_Bow_C" :!type "Actor Class Reference") (`KismetMathLibrary.Conv_ByteToInt` (`self.PartType`))))
  (switch `/Game/TeddyWars/Blueprints/Steve/PartsCrate/PartTypes` (`self.PartType`)
    (:`NewEnumerator0`
      (`SceneComponent.SetRelativeScale3D` (`self.ChildActor`) (0.8 0.8 0.8)))))